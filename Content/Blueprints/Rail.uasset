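; Rail actor that builds a rail mesh along an editable spline and exposes positions along it.
; The construction script tiles spline mesh components in fixed-length sections scaled by actor X scale, clamping tangents to section length to follow the curve.
; GetLocationAtDistance returns a clamped world location, raised by a height offset, plus rotation at a given distance.
; GetRailLength returns the spline's total length.
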(fn `ConstructRail`
  (locals (ScaledSectionLength :type "Float (double-precision)"))
  (bind _returnvalue_x (`KismetMathLibrary.BreakVector` (`self.GetActorScale3D`)))
  (bind _spline (`self.Spline`))
  (set `local.ScaledSectionLength` (* (`self.SectionLength`) _returnvalue_x))
  (for _index (range (+ (`KismetMathLibrary.FTrunc` (/ (`SplineComponent.GetSplineLength` (`self.Spline`)) (`local.ScaledSectionLength`))) 1))
    (bind _returnvalue (`AddComponent|NODE_AddSplineMeshComponent-0`))
    (`SplineMeshComponent.SetForwardAxis` _returnvalue "X" true)
    (bind _returnvalue_2 (* _index (`local.ScaledSectionLength`)))
    (bind _returnvalue_3 (* (+ _index 1) (`local.ScaledSectionLength`)))
    (`SplineMeshComponent.SetStartAndEnd` _returnvalue (`SplineComponent.GetLocationAtDistanceAlongSpline` _spline _returnvalue_2 "Local") (`KismetMathLibrary.ClampVectorSize` (`SplineComponent.GetTangentAtDistanceAlongSpline` _spline _returnvalue_2 "Local") 0.0 (`local.ScaledSectionLength`)) (`SplineComponent.GetLocationAtDistanceAlongSpline` _spline _returnvalue_3 "Local") (`KismetMathLibrary.ClampVectorSize` (`SplineComponent.GetTangentAtDistanceAlongSpline` _spline _returnvalue_3 "Local") 0.0 (`local.ScaledSectionLength`)) true)))

(fn `GetLocationAtDistance`
  (params (Distance :type "Float (double-precision)"))
  (returns (Location :type "Vector Structure") (Rotation :type "Rotator Structure"))
  (bind _spline (`self.Spline`))
  (bind _returnvalue (`KismetMathLibrary.FClamp` Distance 0.0 (`SplineComponent.GetSplineLength` _spline)))
  (return (+ (`SplineComponent.GetLocationAtDistanceAlongSpline` _spline _returnvalue "World") (`KismetMathLibrary.MakeVector` 0.0 0.0 (`self.HeightOffset`))) (`SplineComponent.GetRotationAtDistanceAlongSpline` _spline _returnvalue "World")))

(fn `GetRailLength`
  (returns (ReturnValue :type "Float (double-precision)"))
  (return (`SplineComponent.GetSplineLength` (`self.Spline`))))

(fn `UserConstructionScript`
  (`self.ConstructRail`))