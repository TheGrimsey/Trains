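; Train actor that moves along Rail actors at a set speed, continuing onto each linked NextRail, with networked position sync.
; Server and clients both advance it on Tick; the authority records rail and distance in ServerRailPosition.
; On replication, clients measure drift, including across the next rail, feeding a tenth into each tick's movement.
; They jump when drift exceeds the allowed limit or rails cannot be related.
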(event `self.ReceiveTick`
  (params (DeltaSeconds :type "Float (single-precision)"))
  (if (`self.bMove`)
    (`/Engine/EditorBlueprintResources/StandardMacros.IsValid` (`self.Rail`)
      (:`Is Valid`
        (`self.Move` DeltaSeconds)
        (`/Engine/EditorBlueprintResources/ActorMacros.Switch Has Authority`
          (:`Remote`
            (`KismetSystemLibrary.PrintString` (`KismetStringLibrary.Conv_DoubleToString` (`self.RailDifference`)) true false (struct :`G` 0.66 :`B` 1.0 :`A` 1.0) 0.05)
            (`KismetSystemLibrary.PrintString` (`KismetStringLibrary.Conv_DoubleToString` (- (`GameplayStatics.GetTimeSeconds`) (`GameStateBase.GetServerWorldTimeSeconds` (`GameplayStatics.GetGameState`)))) true false (struct :`G` 0.113437 :`B` 0.171875 :`A` 1.0) 0.05)))))))

(fn `Move`
  (params (DeltaTime :type "Float (double-precision)"))
  (locals (NewRailPosition :type "Float (double-precision)"))
  (`self.MoveToRailPosition` (+ (`self.CurrentRailPosition`) (* (`self.Speed`) DeltaTime) (* (`self.RailDifference`) 0.1))))

(fn `MoveToRailPosition`
  (params (RailPosition :type "Float (double-precision)"))
  (locals (AdjustedRailPosition :type "Float (double-precision)"))
  (bind _returnvalue (`/Game/Blueprints/Rail.GetRailLength` (`self.Rail`)))
  (bind _nextrail (`/Game/Blueprints/Rail.NextRail` (`self.Rail`)))
  (set `local.AdjustedRailPosition` RailPosition)
  (`|ExecutionSequence`
    (:`then_0`
      ;[1 1 1] Handle reaching end of rail
      (if (> (`local.AdjustedRailPosition`) _returnvalue)
        (if (`KismetSystemLibrary.IsValidSoftObjectReference` _nextrail)
          (set `self.Rail` (`|ConvertAsset` _nextrail))
          (set `local.AdjustedRailPosition` (- (`self.CurrentRailPosition`) _returnvalue)))))
    (:`then_1`
      ;[1 1 1] Update Position
      (bind (_location _rotation) (`/Game/Blueprints/Rail.GetLocationAtDistance` (`self.Rail`) (`local.AdjustedRailPosition`)))
      (`self.K2_SetActorLocationAndRotation` _location _rotation)
      ;[1 1 1] Save new position
      (set `self.CurrentRailPosition` (`local.AdjustedRailPosition`)))
    (:`then_2`
      ;[1 1 1] Update networking
      (`/Engine/EditorBlueprintResources/ActorMacros.Switch Has Authority`
        (:`Authority`
          (set `self.ServerRailPosition` (make `/Game/Blueprints/TrainData` (`self.CurrentRailPosition`) (`self.Rail`))))))))

(fn `OnRep_ServerRailPosition`
  (locals (NeedToCorrect :type Boolean) (OnNextRail :type Boolean) (SameRail :type Boolean))
  (bind _serverrailposition_position (break `/Game/Blueprints/TrainData` (`self.ServerRailPosition`)))
  (bind (_serverrailposition_position_2 _serverrailposition_rail) (break `/Game/Blueprints/TrainData` (`self.ServerRailPosition`)))
  (bind _serverrailposition_position_3 (break `/Game/Blueprints/TrainData` (`self.ServerRailPosition`)))
  (bind (_serverrailposition_position_4 _serverrailposition_rail_2) (break `/Game/Blueprints/TrainData` (`self.ServerRailPosition`)))
  (bind (_serverrailposition_position_5 _serverrailposition_rail_3) (break `/Game/Blueprints/TrainData` (`self.ServerRailPosition`)))
  (`/Engine/EditorBlueprintResources/ActorMacros.Switch Has Authority`
    (:`Remote`
      (bind _output_get (set `local.SameRail` (== _serverrailposition_rail_2 (`self.Rail`))))
      (if _output_get
        (set `self.RailDifference` (- _serverrailposition_position (`self.CurrentRailPosition`)))
        (if (> (`KismetMathLibrary.Abs` (`self.RailDifference`)) (`self.AllowedRailDifference`)) :!label _label
          (`self.MoveToRailPosition` (+ (`self.CurrentRailPosition`) (`self.RailDifference`))))
        (else
          (bind _output_get_2 (set `local.OnNextRail` (== (`|ConvertAsset` _serverrailposition_rail_3) (`/Game/Blueprints/Rail.NextRail` (`self.Rail`)))))
          (if _output_get_2
            (set `self.RailDifference` (+ (- (`/Game/Blueprints/Rail.GetRailLength` (`self.Rail`)) (`self.CurrentRailPosition`)) _serverrailposition_position_3))
            (goto _label)
            (else
              ;[1 1 1] Snap to position if we can't figure out the rail distance
              (set `self.Rail` _serverrailposition_rail)
              (`self.MoveToRailPosition` _serverrailposition_position_2))))))))

(fn `SnapToRailPosition`
  (`/Engine/EditorBlueprintResources/StandardMacros.IsValid` (`self.Rail`)
    (:`Is Valid`
      (`self.MoveToRailPosition` (`self.CurrentRailPosition`)))))

(fn `UserConstructionScript`)